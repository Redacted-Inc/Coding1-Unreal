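; BP_EnemySpawnManager coordinates enemy waves across the BP_EnemySpawner actors in the level.
; On BeginPlay it prints a spawner count, with a placeholder for the enemy count.
; NewEnemyWaveCheck looks for remaining BP_Enemy actors and, if none exist, calls SpawningNewEnemies plus a SpawnActor node with no class set.
; SpawningNewEnemies waits briefly, then tells every spawner to SpawnNewEnemy, printing debug progress throughout.
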(event Custom|NewEnemyWaveCheck
  (params (Transform :type Transform))
  (Development|PrintString "Checking enemy count")
  (bind _outactors (Actor|GetAllActorsOfClass "/Game/Blueprints/BP_Enemy.BP_Enemy_C"))
  (if (> (Utilities|Array|Length _outactors) 0)
    (Development|PrintString "There are still more enemies in the level")
    (else
      (CallFunction|SpawningNewEnemies)
      (Game|SpawnActorfromClass "/Game/Blueprints/BP_Key.BP_Key_C" Transform "Undefined" "MultiplyWithRoot" 0 0))))

(event Custom|SpawningNewEnemies
  (Development|PrintString "Spawning new enemies...")
  (Utilities|FlowControl|Delay 4.0)
  (bind _outactors (Actor|GetAllActorsOfClass "/Game/Blueprints/BP_EnemySpawner.BP_EnemySpawner_C"))
  (for (_array_element _array_index) _outactors
    (Default|SpawnNewEnemy _array_element)
    (Development|PrintString (Utilities|String|Append (Utilities|String|ToString(Integer) _array_index) "." (Utilities|GetDisplayName _array_element) " is spawning...")))
  (Development|PrintString "New Wave Complete"))

(event EventBeginPlay
  (Development|PrintString "! SPAWN MANAGER ACTIVE !" true true "(R=0.960417,G=0.843915,B=0.000000,A=1.000000)")
  (bind _outactors (Actor|GetAllActorsOfClass "/Game/Blueprints/BP_EnemySpawner.BP_EnemySpawner_C"))
  ;[0.15 0.15 0.15 0.5] Use this
  (Development|PrintString (Utilities|String|Append "There are " (Utilities|String|ToString(Integer) (Utilities|Array|Length _outactors)) " spawners in the level." " There are " "##" " Enemies in the level") true true "(R=0.852083,G=0.021488,B=0.000000,A=1.000000)"))

(fn ConstructionScript)