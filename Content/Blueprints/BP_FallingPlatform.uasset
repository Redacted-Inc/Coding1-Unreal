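; BP_FallingPlatform is a platform that falls a short delay after the third-person character steps on its trigger box, then returns to its starting transform.
; An IsReady flag gates a chain of Activate, Falling and Reset events, each swapping the platform's material to show its state.
; The fall uses physics simulation; Reset disables it and a timeline lerps the platform back before re-arming it.
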(event OnComponentBeginOverlap(BoxTrigger)
  (params (OverlappedComponent :type Primitive%20Component%20Object%20Reference) (OtherActor :type Actor%20Object%20Reference) (OtherComp :type Primitive%20Component%20Object%20Reference) (OtherBodyIndex :type Integer) (bFromSweep :type Boolean) (SweepResult :type Hit%20Result%20Structure%20%28by%20ref%29))
  (if (Variables|Default|GetIsReady)
    (Development|PrintString "Help! I'm being stepped on")
    (Utilities|Casting|CastToBP_ThirdPersonCharacter OtherActor)
    (Variables|Default|SetIsReady false)
    (CallFunction|Activate)))

(event Custom|Reset
  (Development|PrintString "Reseting...")
  (Rendering|Material|SetMaterial (Variables|Default|GetPlatform) 0 "/Game/Materials/FallingPlatform/MI_Resetting.MI_Resetting")
  (Physics|SetSimulatePhysics (Variables|Default|GetPlatform) false)
  (Variables|Default|SetFallenPosition (Transformation|GetWorldTransform (Variables|Default|GetPlatform)))
  (bind _newtrack_0 (Timeline|GoBackToStartTransform PlayFromStart)
    (:Update
      (Transformation|SetWorldTransform (Variables|Default|GetPlatform) (Math|Transform|Lerp(Transform) (Variables|Default|GetFallenPosition) (Variables|Default|GetStartingTransform) _newtrack_0) false false))
    (:Finished
      (Variables|Default|SetIsReady true)
      (Rendering|Material|SetMaterial (Variables|Default|GetPlatform) 0 "/Game/Materials/FallingPlatform/MI_ReadyPlatform.MI_ReadyPlatform"))))

(event Custom|Activate
  (Development|PrintString "Uh oh...")
  (Rendering|Material|SetMaterial (Variables|Default|GetPlatform) 0 "/Game/Materials/FallingPlatform/MI_Active.MI_Active")
  (Utilities|FlowControl|Delay (Variables|PlatformSetting|GetFallDelayDuration))
  (CallFunction|Falling))

(event Custom|Falling
  (Development|PrintString "WAAAAAAAAAAAAAAAAAAAAAAAAAAAAAAAAAAAAAAAAAA")
  (Rendering|Material|SetMaterial (Variables|Default|GetPlatform) 0 "/Game/Materials/FallingPlatform/MI_Falling.MI_Falling")
  (Physics|SetSimulatePhysics (Variables|Default|GetPlatform) true)
  (Utilities|FlowControl|Delay (Variables|PlatformSetting|GetResetDelayDuration))
  (CallFunction|Reset))

(event EventBeginPlay
  (Variables|Default|SetStartingTransform (Transformation|GetWorldTransform (Variables|Default|GetPlatform)))
  (Rendering|Material|SetMaterial (Variables|Default|GetPlatform) 0 "/Game/Materials/FallingPlatform/MI_ReadyPlatform.MI_ReadyPlatform"))

(fn ConstructionScript)