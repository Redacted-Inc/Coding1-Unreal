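; Elevator platform that travels between Start and End transforms when the third-person character steps into its Box trigger.
; One timeline plays forward or reversed according to AtTop, lerping the transform, with IsReady blocking retriggers mid-move.
; CallTop and CallBottom triggers summon it from its current transform using their own timelines.
; Timeline event tracks swap platform materials to show state; older elevator logic remains unconnected.
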(event OnComponentBeginOverlap(Box)
  (params (OverlappedComponent :type Primitive%20Component%20Object%20Reference) (OtherActor :type Actor%20Object%20Reference) (OtherComp :type Primitive%20Component%20Object%20Reference) (OtherBodyIndex :type Integer) (bFromSweep :type Boolean) (SweepResult :type Hit%20Result%20Structure%20%28by%20ref%29))
  (Utilities|Casting|CastToBP_ThirdPersonCharacter OtherActor)
  (if (Variables|Default|GetIsReady)
    (Variables|Default|SetIsReady false)
    (if (Variables|Default|GetAtTop)
      (Development|PrintString "Going Up")
      (Variables|Default|SetAtTop false)
      (bind _newtrack_0 (Timeline|GoDown ReverseFromEnd)
        (:Update
          (Transformation|SetWorldLocationAndRotation (Variables|Default|GetPlatform) (.location (Math|Transform|Lerp(Transform) (Transformation|GetWorldTransform (Variables|Default|GetEnd)) (Transformation|GetWorldTransform (Variables|Default|GetStart)) _newtrack_0)) (.rotation (Math|Transform|Lerp(Transform) (Transformation|GetWorldTransform (Variables|Default|GetEnd)) (Transformation|GetWorldTransform (Variables|Default|GetStart)) _newtrack_0)) false false))
        (:Finished
          (Variables|Default|SetIsReady true))
        (:Ready
          (Rendering|Material|SetMaterial (Variables|Default|GetPlatform) 0 "/Game/Materials/FallingPlatform/MI_Active.MI_Active"))
        (:Moving
          (Rendering|Material|SetMaterial (Variables|Default|GetPlatform) 0 "/Game/Materials/FallingPlatform/MI_Resetting.MI_Resetting"))
        (:Stopped
          (Rendering|Material|SetMaterial (Variables|Default|GetPlatform) 0 "/Game/Materials/FallingPlatform/MI_Falling.MI_Falling")))
      (else
        (Development|PrintString "Going Down")
        (Variables|Default|SetAtTop true)
        (Timeline|GoDown PlayFromStart)))))

(event OnComponentBeginOverlap(CallBottom)
  (params (OverlappedComponent :type Primitive%20Component%20Object%20Reference) (OtherActor :type Actor%20Object%20Reference) (OtherComp :type Primitive%20Component%20Object%20Reference) (OtherBodyIndex :type Integer) (bFromSweep :type Boolean) (SweepResult :type Hit%20Result%20Structure%20%28by%20ref%29))
  (if (Variables|Default|GetIsReady)
    (Variables|Default|SetIsReady false)
    (Variables|Default|SetAtTop true)
    (Variables|Default|SetCurrentPosition (Transformation|GetWorldTransform (Variables|Default|GetPlatform)))
    (bind _newtrack_0 (Timeline|CallBottomTime PlayFromStart)
      (:Update
        (Transformation|SetWorldLocationAndRotation (Variables|Default|GetPlatform) (.location (Math|Transform|Lerp(Transform) (Variables|Default|GetCurrentPosition) (Transformation|GetWorldTransform (Variables|Default|GetStart)) _newtrack_0)) (.rotation (Math|Transform|Lerp(Transform) (Variables|Default|GetCurrentPosition) (Transformation|GetWorldTransform (Variables|Default|GetStart)) _newtrack_0)) false false))
      (:Finished
        (Variables|Default|SetIsReady true))
      (:Moving
        (Rendering|Material|SetMaterial (Variables|Default|GetPlatform) 0 "/Game/Materials/FallingPlatform/MI_Resetting.MI_Resetting"))
      (:Ready
        (Rendering|Material|SetMaterial (Variables|Default|GetPlatform) 0 "/Game/Materials/FallingPlatform/MI_Active.MI_Active"))
      (:Stopped
        (Rendering|Material|SetMaterial (Variables|Default|GetPlatform) 0 "/Game/Materials/FallingPlatform/MI_Falling.MI_Falling")))))

(event OnComponentBeginOverlap(CallTop)
  (params (OverlappedComponent :type Primitive%20Component%20Object%20Reference) (OtherActor :type Actor%20Object%20Reference) (OtherComp :type Primitive%20Component%20Object%20Reference) (OtherBodyIndex :type Integer) (bFromSweep :type Boolean) (SweepResult :type Hit%20Result%20Structure%20%28by%20ref%29))
  (if (Variables|Default|GetIsReady)
    (Variables|Default|SetIsReady false)
    (Variables|Default|SetAtTop false)
    (Variables|Default|SetCurrentPosition (Transformation|GetWorldTransform (Variables|Default|GetPlatform)))
    (bind _newtrack_0 (Timeline|CallTopTime PlayFromStart)
      (:Update
        (Transformation|SetWorldLocationAndRotation (Variables|Default|GetPlatform) (.location (Math|Transform|Lerp(Transform) (Variables|Default|GetCurrentPosition) (Transformation|GetWorldTransform (Variables|Default|GetEnd)) _newtrack_0)) (.rotation (Math|Transform|Lerp(Transform) (Variables|Default|GetCurrentPosition) (Transformation|GetWorldTransform (Variables|Default|GetEnd)) _newtrack_0)) false false))
      (:Finished
        (Variables|Default|SetIsReady true))
      (:Ready
        (Rendering|Material|SetMaterial (Variables|Default|GetPlatform) 0 "/Game/Materials/FallingPlatform/MI_Active.MI_Active"))
      (:Moving
        (Rendering|Material|SetMaterial (Variables|Default|GetPlatform) 0 "/Game/Materials/FallingPlatform/MI_Resetting.MI_Resetting"))
      (:Stopped
        (Rendering|Material|SetMaterial (Variables|Default|GetPlatform) 0 "/Game/Materials/FallingPlatform/MI_Falling.MI_Falling")))))

(event EventBeginPlay)

(fn ConstructionScript)